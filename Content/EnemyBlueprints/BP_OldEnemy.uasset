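; Hammer-throwing enemy that chases the player and attacks when in range with line of sight.
; Tick faces the player, traces forward for sight and holds the spawned BP_HammerEnemy in front until thrown; throws need a caught hammer and random cooldown.
; A looping AIMoveTo uses attack range as acceptance radius, dropping to zero when sight is lost.
; A separate event stops an AIController and briefly enables box physics.
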(event Custom|ChangeCollisionsToPhysics
  (bind _returnvalue (Actor|GetActorOfClass "/Script/AIModule.AIController"))
  (AI|Navigation|StopMovement _returnvalue)
  (Physics|SetSimulatePhysics (Variables|Default|GetBox) true)
  (Collision|SetCollisionEnabled (Variables|Default|GetBox) "QueryAndPhysics")
  (Utilities|FlowControl|Delay 0.2)
  (Physics|SetSimulatePhysics (Variables|Default|GetBox) false)
  (Collision|SetCollisionEnabled (Variables|Default|GetBox) "QueryOnly"))

(event Custom|StartMovement
  (AI|AIMoveTo self "0, 0, 0" (Variables|Default|Getplayer) (Variables|Default|GetcurrentDistance) false :!label _label
    (:OnSuccess
      _)
    (:OnFail
      _))
  (Utilities|FlowControl|Delay 1.0)
  (goto _label))

(event Custom|CreateHammer
  (bind _returnvalue (Game|SpawnActorfromClass "/Game/EnemyBlueprints/BP_HammerEnemy.BP_HammerEnemy_C" (Math|Transform|MakeTransform (+ (.location (Transformation|GetActorTransform)) (* (Math|Vector|GetForwardVector (Transformation|GetWorldRotation (Variables|Default|GetBox))) 1e+02)) (Math|Conversions|RotationFromXVector (Math|Vector|GetForwardVector (Transformation|GetWorldRotation (Variables|Default|GetBox)))) "1.000000,1.000000,1.000000") "Undefined" "MultiplyWithRoot" 0 0))
  (bind _output_get (Variables|Default|Sethammer _returnvalue))
  (Default|SetParent _output_get self))

(event Custom|CheckSight
  (bind _returnvalue (Transformation|GetActorTransform))
  (bind _outhit (Collision|LineTraceByChannel (.location _returnvalue) (+ (.location _returnvalue) (* (Math|Vector|GetForwardVector (Transformation|GetWorldRotation (Variables|Default|GetBox))) (Variables|Default|GetattackDistance))) "TraceTypeQuery1" false (Utilities|Array|MakeArray (Variables|Default|GetHammer)) "ForOneFrame"))
  (Utilities|Casting|CastToBP_player (.hitactor _outhit)
    (:then
      (Variables|Default|SetcurrentDistance (Variables|Default|GetattackDistance))
      (Variables|Default|SetseePlayer true))
    (:CastFailed
      (Variables|Default|SetcurrentDistance 0.0)
      (Variables|Default|SetseePlayer false))))

(event Custom|Attack
  (if (Variables|Default|GetcanAttack)
    (if (Variables|/Game/EnemyBlueprints/BP_SledgeHammer.BP_SledgeHammer_C|GethasCaught (Variables|Default|GetHammer))
      (Default|Shoot (Variables|Default|GetHammer) (Math|Vector|GetForwardVector (Transformation|GetWorldRotation (Variables|Default|GetGC_Cube))))
      (Variables|Default|SetcanAttack false)
      (Utilities|FlowControl|Delay (Math|Random|RandomFloatinRange 1.0 2.0))
      (Variables|Default|SetcanAttack true))))

(event Custom|RotateHammer
  (Utilities|IsValid (Variables|Default|Gethammer)
    (:Is%20Valid
      (if (not (Variables|/Game/EnemyBlueprints/BP_SledgeHammer.BP_SledgeHammer_C|GetisFlying (Variables|Default|Gethammer)))
        (Transformation|SetActorTransform (Variables|Default|Gethammer) (Math|Transform|MakeTransform (+ (.location (Transformation|GetActorTransform)) (* (Math|Vector|GetForwardVector (Transformation|GetWorldRotation (Variables|Default|GetBox))) 2e+02)) (Math|Conversions|RotationFromXVector (Math|Vector|GetForwardVector (Transformation|GetWorldRotation (Variables|Default|GetBox)))) "1.000000,1.000000,1.000000"))))))

(event EventBeginPlay
  (Variables|Default|SetcurrentDistance (Variables|Default|GetattackDistance))
  (Variables|Default|SetHealth (Variables|Default|GetMaxHealth))
  (Variables|Default|SetBody (Variables|Default|GetGC_Cube))
  (bind _outactors (Actor|GetAllActorsOfClass "/Game/FirstPerson/Blueprints/BP_player.BP_player_C"))
  (Variables|Default|Setplayer (Utilities|Array|Get(acopy) _outactors))
  (CallFunction|StartMovement)
  (CallFunction|CreateHammer))

(event EventTick
  (params (DeltaSeconds :type Float%20%28single-precision%29))
  (Utilities|IsValid (Variables|Default|Getplayer)
    (:Is%20Valid
      (Transformation|SetActorRotation (Math|Conversions|RotationFromXVector (- (Transformation|GetActorLocation (Variables|Default|Getplayer)) (Transformation|GetActorLocation))))
      (CallFunction|CheckSight)
      (CallFunction|RotateHammer)
      (if (and (<= (Transformation|GetDistanceTo (Variables|Default|Getplayer) self) (Variables|Default|GetattackDistance)) (Variables|Default|GetseePlayer))
        (CallFunction|Attack)))))

(event EventDie
  (Actor|DestroyActor (Variables|Default|GetHammer))
  (Actor|DestroyActor))

(fn ConstructionScript)