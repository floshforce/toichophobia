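; BP_LevelPortal is an interactable portal that moves the player to another level.
; A box trigger shows a widget while something overlaps it and hides it otherwise, starting hidden on BeginPlay.
; On Interaction, it stores its level tag in the GI_Main game instance so the value survives the map change, then opens the configured level by name.
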(event OnComponentBeginOverlap(Box)
  (params (OverlappedComponent :type Primitive%20Component%20Object%20Reference) (OtherActor :type Actor%20Object%20Reference) (OtherComp :type Primitive%20Component%20Object%20Reference) (OtherBodyIndex :type Integer) (bFromSweep :type Boolean) (SweepResult :type Hit%20Result%20Structure%20%28by%20ref%29))
  (Rendering|SetVisibility (Variables|Default|GetWidget) true false))

(event OnComponentEndOverlap(Box)
  (params (OverlappedComponent :type Primitive%20Component%20Object%20Reference) (OtherActor :type Actor%20Object%20Reference) (OtherComp :type Primitive%20Component%20Object%20Reference) (OtherBodyIndex :type Integer))
  (Rendering|SetVisibility (Variables|Default|GetWidget) false false))

(event EventBeginPlay
  (Rendering|SetVisibility (Variables|Default|GetWidget) false false))

(event EventInteraction
  (bind _asgi_main (Utilities|Casting|CastToGI_Main (Game|GetGameInstance)))
  (Variables|/Game/House_maps/GI_Main.GI_Main_C|SetLevelTag _asgi_main (Variables|Default|GetLeve%20Tag))
  (Game|OpenLevel(byName) (Variables|Default|GetLevelName)))

(fn ConstructionScript)