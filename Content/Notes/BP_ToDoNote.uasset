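; BP_ToDoNote is a readable to-do note the player can pick up and put down.
; Its InteractionRange overlap shows or hides a prompt Widget.
; Interaction uses a FlipFlop: picking up plays a sound, opens WB_ToDoNote, blocks look and move input, and hides the note.
; Putting down calls PutDownNote on that widget, restores input, and shows the note again after a short delay.
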(event OnComponentBeginOverlap(InteractionRange)
  (params (OverlappedComponent :type Primitive%20Component%20Object%20Reference) (OtherActor :type Actor%20Object%20Reference) (OtherComp :type Primitive%20Component%20Object%20Reference) (OtherBodyIndex :type Integer) (bFromSweep :type Boolean) (SweepResult :type Hit%20Result%20Structure%20%28by%20ref%29))
  (Rendering|SetVisibility (Variables|Default|GetWidget) true false))

(event OnComponentEndOverlap(InteractionRange)
  (params (OverlappedComponent :type Primitive%20Component%20Object%20Reference) (OtherActor :type Actor%20Object%20Reference) (OtherComp :type Primitive%20Component%20Object%20Reference) (OtherBodyIndex :type Integer))
  (Rendering|SetVisibility (Variables|Default|GetWidget) false false))

(event EventBeginPlay
  (Rendering|SetVisibility (Variables|Default|GetWidget) false false))

(event EventInteraction
  (bind _returnvalue (Game|GetPlayerController 0))
  (bind _note (Variables|Default|GetNote))
  (bind _note_2 (Variables|Default|GetNote))
  (bind _returnvalue_2 (Transformation|GetWorldLocation _note))
  (Utilities|FlowControl|FlipFlop
    (:A
      (Audio|PlaySoundatLocation "/Game/Notes/PickUp_Sound.PickUp_Sound" _returnvalue_2 "0, 0, 0" 1.0 1.0 0.0 0 0 0 0)
      (bind _returnvalue_3 (UserInterface|CreateWidget "/Game/Notes/WB_ToDoNote.WB_ToDoNote_C"))
      (UserInterface|Viewport|AddtoViewport _returnvalue_3 0)
      (Input|SetIgnoreLookInput _returnvalue true)
      (Input|SetIgnoreMoveInput _returnvalue true)
      (Rendering|SetVisibility _note_2 false false))
    (:B
      (Audio|PlaySoundatLocation "/Game/Notes/PutDown_Sound.PutDown_Sound" _returnvalue_2 "0, 0, 0" 1.0 1.0 0.0 0 0 0 0)
      (Default|PutDownNote _returnvalue_3)
      (Input|SetIgnoreLookInput _returnvalue false)
      (Input|SetIgnoreMoveInput _returnvalue false)
      (Utilities|FlowControl|Delay 0.8)
      (Rendering|SetVisibility _note_2 true false))))

(fn ConstructionScript)