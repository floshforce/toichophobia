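; Ranged enemy that chases the player and launches a spawned BP_HammerEnemy at them.
; Each tick it faces the player, line-traces for sight, holds the hammer ahead and shoots when in range, with a random cooldown.
; A looping AIMoveTo uses attack range as acceptance radius when the player is visible, zero otherwise.
; Damage swaps crack materials; death at exactly zero health removes hammer and actor, while a separate event shatters the geometry-collection body.
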(event Custom|TurnOnDestractability
  (Collision|SetCollisionEnabled (Variables|Default|GetCapsuleComponent) "NoCollision")
  (Physics|SetSimulatePhysics (Variables|Default|GetGC_Cube) true)
  (Collision|SetCollisionEnabled (Variables|Default|GetGC_Cube) "QueryAndPhysics")
  (Physics|AddRadialImpulse (Variables|Default|GetGC_Cube) (Transformation|GetActorLocation) 1e+03 1e+04 "RIF_Constant" false))

(event Custom|StartMovement
  ;[0.15 0.15 0.15 0.5] Nav
  (AI|AIMoveTo self "0, 0, 0" (Variables|Default|Getplayer) (Variables|Default|GetcurrentDistance) false :!label _label
    (:OnSuccess
      _)
    (:OnFail
      _))
  (Utilities|FlowControl|Delay 1.0)
  (goto _label))

(event Custom|CreateHammer
  ;[0.15 0.15 0.15 0.5] Hammer
  (bind _returnvalue (Game|SpawnActorfromClass "/Game/EnemyBlueprints/BP_HammerEnemy.BP_HammerEnemy_C" (Math|Transform|MakeTransform (+ (.location (Transformation|GetActorTransform)) (* (Math|Vector|GetForwardVector (Transformation|GetWorldRotation (Variables|Default|GetCapsuleComponent))) 1e+02)) (Math|Conversions|RotationFromXVector (Math|Vector|GetForwardVector (Transformation|GetWorldRotation (Variables|Default|GetCapsuleComponent)))) "1.000000,1.000000,1.000000") "Undefined" "MultiplyWithRoot" 0 0))
  (bind _output_get (Variables|Default|Sethammer _returnvalue))
  (Default|SetParent _output_get self))

(event Custom|CheckSight
  (bind _returnvalue (Transformation|GetActorTransform))
  ;[0.15 0.15 0.15 0.5] Nav
  (bind _outhit (Collision|LineTraceByChannel (.location _returnvalue) (+ (.location _returnvalue) (* (Math|Vector|GetForwardVector (Transformation|GetWorldRotation (Variables|Default|GetCapsuleComponent))) (Variables|Default|GetattackDistance))) "TraceTypeQuery1" false (Utilities|Array|MakeArray (Variables|Default|GetHammer) 0) "ForOneFrame"))
  (Utilities|Casting|CastToBP_player (.hitactor _outhit)
    (:then
      (Variables|Default|SetcurrentDistance (Variables|Default|GetattackDistance))
      (Variables|Default|SetseePlayer true))
    (:CastFailed
      (Variables|Default|SetcurrentDistance 0.0)
      (Variables|Default|SetseePlayer false))))

(event Custom|Attack
  (Utilities|IsValid (Variables|Default|GetHammer)
    (:Is%20Valid
      (if (Variables|Default|GetcanAttack)
        (if (Variables|/Game/EnemyBlueprints/BP_SledgeHammer.BP_SledgeHammer_C|GethasCaught (Variables|Default|GetHammer))
          (Default|Shoot (Variables|Default|GetHammer) (Math|Vector|GetForwardVector (Transformation|GetWorldRotation (Variables|Default|GetGC_Cube))))
          (Variables|Default|SetcanAttack false)
          (Utilities|FlowControl|Delay (Math|Random|RandomFloatinRange 3.0 4.0))
          (Variables|Default|SetcanAttack true))))))

(event Custom|Die
  (Actor|DestroyActor (Variables|Default|Gethammer))
  (Variables|Default|SetisDead true)
  (Utilities|FlowControl|Delay 5.0)
  (Actor|DestroyActor))

(event Custom|RotateHammer
  ;[0.15 0.15 0.15 0.5] Hammer
  (Utilities|IsValid (Variables|Default|Gethammer)
    (:Is%20Valid
      (if (not (Variables|/Game/EnemyBlueprints/BP_SledgeHammer.BP_SledgeHammer_C|GetisFlying (Variables|Default|Gethammer)))
        (Transformation|SetActorTransform (Variables|Default|Gethammer) (Math|Transform|MakeTransform (+ (.location (Transformation|GetActorTransform)) (* (Math|Vector|GetForwardVector (Transformation|GetWorldRotation (Variables|Default|GetCapsuleComponent))) 2e+02)) (Math|Conversions|RotationFromXVector (Math|Vector|GetForwardVector (Transformation|GetWorldRotation (Variables|Default|GetCapsuleComponent)))) "1.000000,1.000000,1.000000"))))))

(event EventBeginPlay
  (Variables|Default|SetcurrentDistance (Variables|Default|GetattackDistance))
  (Variables|Default|SetHealth (Variables|Default|GetMaxHealth))
  (Variables|Default|SetBody (Variables|Default|GetGC_Cube))
  (bind _outactors (Actor|GetAllActorsOfClass "/Game/FirstPerson/Blueprints/BP_player.BP_player_C"))
  (Variables|Default|Setplayer (Utilities|Array|Get(acopy) _outactors))
  (CallFunction|StartMovement)
  (CallFunction|CreateHammer))

(event EventTick
  (params (DeltaSeconds :type Float%20%28single-precision%29))
  (if (not (Variables|Default|GetisDead))
    (Utilities|IsValid (Variables|Default|Getplayer)
      (:Is%20Valid
        (Transformation|SetActorRotation (Math|Conversions|RotationFromXVector (- (Transformation|GetActorLocation (Variables|Default|Getplayer)) (Transformation|GetActorLocation))))
        (CallFunction|CheckSight)
        (CallFunction|RotateHammer)
        (if (and (<= (Transformation|GetDistanceTo (Variables|Default|Getplayer) self) (Variables|Default|GetattackDistance)) (Variables|Default|GetseePlayer))
          (CallFunction|Attack))))))

(event EventTakeDamage
  (params (value :type Integer))
  ;[0.15 0.15 0.15 0.5] Health
  (Variables|Default|Sethealth (- (Variables|Default|Gethealth) value))
  (if (== (Variables|Default|Gethealth) 0)
    (CallFunction|Die)
    (elif (< (Variables|Default|Gethealth) (- (Variables|Default|GetmaxHealth) (* (/ (Variables|Default|GetmaxHealth) (+ (Utilities|Array|Length (Variables|Default|GetcrackMaterials)) 1)) (+ (Variables|Default|GetcurrentMaterialIndex) 1))))
      (Rendering|Material|SetMaterial (Variables|Default|GetBody) 0 (Utilities|Array|Get(acopy) (Variables|Default|GetcrackMaterials) (Variables|Default|GetcurrentMaterialIndex)))
      (Math|Integer|IncrementInt (Variables|Default|GetcurrentMaterialIndex)))))

(fn ConstructionScript
  (|CallParentFunction))