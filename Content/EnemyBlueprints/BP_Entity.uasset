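; BP_Entity is a damageable entity that shows cracks as it loses health and destroys itself on death.
; It starts at MaxHealth with the Cube as its Body, and TakeDamage subtracts from Health, calling Die only when Health equals exactly zero.
; Otherwise, MaxHealth is split evenly across CrackMaterials, and Body advances at most one material per hit when Health falls below the next threshold.
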(event Custom|Die
  (Actor|DestroyActor))

(event EventBeginPlay
  (Variables|Default|SetHealth (Variables|Default|GetMaxHealth))
  (Variables|Default|SetBody (Variables|Default|GetCube)))

(event EventTakeDamage
  (params (value :type Integer))
  (Variables|Default|SetHealth (- (Variables|Default|GetHealth) value))
  (if (== (Variables|Default|GetHealth) 0)
    (CallFunction|Die)
    (elif (< (Variables|Default|GetHealth) (- (Variables|Default|GetMaxHealth) (* (/ (Variables|Default|GetMaxHealth) (Utilities|Array|Length (Variables|Default|GetCrackMaterials))) (+ (Variables|Default|GetcurrentMaterialIndex) 1))))
      (Rendering|Material|SetMaterial (Variables|Default|GetBody) 0 (Utilities|Array|Get(acopy) (Variables|Default|GetCrackMaterials) (+ (Variables|Default|GetcurrentMaterialIndex) 1)))
      (Math|Integer|IncrementInt (Variables|Default|GetcurrentMaterialIndex)))))

(fn ConstructionScript)