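; BP_enemyMelee is a melee enemy whose attack is a forward dash that damages and knocks back the player.
; Attack disables movement, zeroes braking friction and uses a looping timer to repeatedly launch the enemy forward.
; A capsule hit on the player during the dash ends it, deals damage and launches the player forward and upward for a short time.
; Dash exit restores friction and movement, then re-arms attacking after a randomised cooldown.
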(event OnComponentHit(CapsuleComponent)
  (params (HitComponent :type Primitive%20Component%20Object%20Reference) (OtherActor :type Actor%20Object%20Reference) (OtherComp :type Primitive%20Component%20Object%20Reference) (NormalImpulse :type Vector :default "0, 0, 0") (Hit :type Hit%20Result%20Structure%20%28by%20ref%29))
  (Utilities|Casting|CastToBP_player OtherActor)
  (if (and (Variables|Default|GetisDashing) (!= (Variables|Default|GetotherIsFlying) true))
    (Development|PrintText "HIIIIIIIIIIIIIIIIIIIIIIIIT")
    (Variables|Default|SetotherIsFlying true)
    (CallFunction|ExitDash)
    (Default|TakeDamage (Variables|Default|Getplayer) 2)
    (Variables|/Script/Engine.CharacterMovementComponent|SetBrakingFrictionFactor (Variables|Character|GetCharacterMovement) 0.0)
    (bind _returnvalue (Utilities|Time|SetTimerbyEvent (delegate Custom|ApplyLaunchToOther) 0.02 true))
    (Utilities|FlowControl|Delay 0.6)
    (Utilities|Time|PauseTimerbyHandle _returnvalue)
    (Variables|/Script/Engine.CharacterMovementComponent|SetBrakingFrictionFactor (Variables|Character|GetCharacterMovement) 1.0)
    (Variables|Default|SetotherIsFlying false)))

(event Custom|ExitDash
  (Utilities|Time|PauseTimerbyHandle (Variables|Default|GetlaunchTimer))
  (Variables|/Script/Engine.CharacterMovementComponent|SetBrakingFrictionFactor (Variables|Character|GetCharacterMovement) 1.0)
  (Variables|Default|SetisDashing false)
  (Utilities|FlowControl|Delay 1.0)
  (CallFunction|EnableMovement)
  (Utilities|FlowControl|Delay (Math|Random|RandomFloatinRange 1.0 2.0))
  (Variables|Default|SetcanAttack true))

(event Custom|ApplyLaunchToSelf
  (Character|LaunchCharacter (* (Math|Vector|GetForwardVector (Variables|Default|GetCapsuleComponent)) (Variables|Default|GetdashStrength)) true true))

(event Custom|ApplyLaunchToOther
  (Character|LaunchCharacter (Variables|Default|Getplayer) (* (+ (Math|Vector|GetForwardVector (Variables|Default|GetCapsuleComponent)) (* (Math|Vector|VectorUp) 0.3)) (* (Variables|Default|GetdashStrength) 0.7)) true true))

(event EventBeginPlay
  (CallFunction|SetupBase))

(event EventTick
  (params (DeltaSeconds :type Float%20%28single-precision%29))
  (CallFunction|OnTickBase))

(event EventAttack
  (if (Variables|Default|GetcanAttack)
    (Variables|Default|SetcanAttack false)
    (Variables|Default|SetisDashing true)
    (CallFunction|DisableMovement)
    (Variables|/Script/Engine.CharacterMovementComponent|SetBrakingFrictionFactor (Variables|Character|GetCharacterMovement) 0.0)
    (bind _returnvalue (Utilities|Time|SetTimerbyEvent (delegate Custom|ApplyLaunchToSelf) 0.02 true))
    (Variables|Default|SetlaunchTimer _returnvalue)
    (if (Variables|Default|GetisDashing)
      (Utilities|FlowControl|Delay 1.2)
      (CallFunction|ExitDash))))

(fn ConstructionScript
  (|CallParentFunction))