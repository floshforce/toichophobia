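; Thrown sledgehammer projectile in the enemy Blueprints that flies out, damages what it hits and homes back to its parent like a boomerang.
; Shoot launches it straight along a direction, and Return switches on homing after hitting an IDamagable or after a one-second miss.
; While homing, Tick turns it relative to the parent and catches it within range, stopping movement and collision.
; Non-parent overlaps briefly disable collision.
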(event OnComponentBeginOverlap(Box)
  (params (OverlappedComponent :type Primitive%20Component%20Object%20Reference) (OtherActor :type Actor%20Object%20Reference) (OtherComp :type Primitive%20Component%20Object%20Reference) (OtherBodyIndex :type Integer) (bFromSweep :type Boolean) (SweepResult :type Hit%20Result%20Structure%20%28by%20ref%29))
  (CallFunction|Debug)
  (Variables|Default|SetcollisionActor OtherActor)
  (if (not (== OtherActor (Variables|Default|Getparent)))
    (CallFunction|DisableCollision)
    (if (Utilities|DoesObjectImplementInterface (Variables|Default|GetcollisionActor) "/Game/EnemyBlueprints/IDamagable.IDamagable_C")
      (Class|IDamagable|TakeDamage(Message) (Variables|Default|GetcollisionActor) (Variables|Default|Getdamage))
      (Variables|Default|SethasHitSomething true)
      (CallFunction|Return))))

(event Custom|Shoot
  (params (direction :type Vector))
  (if (Variables|Default|GethasCaught)
    (Variables|Default|SetisFlying true)
    (Variables|Default|SethasHitSomething false)
    (Transformation|SetActorRotation (Math|Conversions|RotationFromXVector direction))
    (Variables|/Script/Engine.ProjectileMovementComponent|SetbIsHomingProjectile (Variables|Default|GetProjectileMovementForward) false)
    (Collision|SetCollisionEnabled (Variables|Default|GetBox) "QueryAndPhysics")
    (Components|Activation|Activate (Variables|Default|GetProjectileMovementForward) true)
    (Variables|/Script/Engine.MovementComponent|SetVelocity (Variables|Default|GetProjectileMovementForward) (* (Math|Vector|GetForwardVector (Variables|Default|GetBox)) (Class|MovementComponent|GetMaxSpeed (Variables|Default|GetProjectileMovementForward))))
    (Utilities|FlowControl|Delay 1.0)
    (if (not (Variables|Default|GethasHitSomething))
      (CallFunction|Return))))

(event Custom|Return
  (Variables|Default|SethasCaught false)
  (Variables|/Script/Engine.ProjectileMovementComponent|SetbIsHomingProjectile (Variables|Default|GetProjectileMovementForward) true)
  (Variables|/Script/Engine.ProjectileMovementComponent|SetHomingTargetComponent (Variables|Default|GetProjectileMovementForward) (Variables|/Script/Engine.Actor|GetRootComponent (Variables|Default|Getparent))))

(event Custom|SetParent
  (params (parent :type Actor%20Object%20Reference))
  (bind _output_get (Variables|Default|Setparent parent))
  (Variables|/Script/Engine.ProjectileMovementComponent|SetHomingTargetComponent (Variables|Default|GetProjectileMovementForward) (Variables|/Script/Engine.Actor|GetRootComponent _output_get)))

(event Custom|Catch
  (if (not (Variables|Default|GethasCaught))
    (Variables|Default|SetisFlying false)
    (Variables|/Script/Engine.ProjectileMovementComponent|SetbIsHomingProjectile (Variables|Default|GetProjectileMovementForward) false)
    (Components|Activation|Deactivate (Variables|Default|GetProjectileMovementForward))
    (Variables|Default|SethasCaught true)
    (Variables|/Script/Engine.MovementComponent|SetVelocity (Variables|Default|GetProjectileMovementForward) "0, 0, 0")
    (Collision|SetCollisionEnabled (Variables|Default|GetBox) "NoCollision")))

(event Custom|Debug
  (Development|PrintText (Utilities|Text|ToText(String) (Utilities|String|EnumtoString (Collision|GetCollisionEnabled (Variables|Default|GetBox))))))

(event Custom|RotateTo
  (Transformation|SetActorRotation (Math|Interpolation|RInterpTo (Transformation|GetActorRotation) (Math|Rotator|FindLookatRotation (Transformation|GetActorLocation (Variables|Default|Getparent)) (Transformation|GetActorLocation)) (Utilities|Time|GetWorldDeltaSeconds) 5.0)))

(event Custom|DisableCollision
  (Collision|SetCollisionEnabled (Variables|Default|GetBox) "NoCollision")
  (Utilities|FlowControl|Delay 0.1)
  (Collision|SetCollisionEnabled (Variables|Default|GetBox) "QueryAndPhysics"))

(event EventTick
  (params (DeltaSeconds :type Float%20%28single-precision%29))
  (if (Variables|/Script/Engine.ProjectileMovementComponent|GetbIsHomingProjectile (Variables|Default|GetProjectileMovementForward))
    (CallFunction|Rotateto)
    (if (< (Transformation|GetDistanceTo (Variables|Default|Getparent) self) 5e+02)
      (CallFunction|Catch))))

(event EventBeginPlay
  (Variables|Default|Setdamage 1)
  (Components|Activation|SetActive (Variables|Default|GetProjectileMovementForward) false true))

(fn ConstructionScript)