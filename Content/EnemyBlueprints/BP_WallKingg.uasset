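; Wall King enemy that carries a spawned BP_HammerBoss and alternates randomly between a dash and a hammer throw.
; Attack fires only while the hammer is caught, with random delays re-arming it; Tick pins the hammer in front unless it is flying.
; Looping timers repeatedly call LaunchCharacter to drive the dash and, on capsule contact, to knock the damaged player up and away.
; Death destroys the hammer before running the parent's logic.
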(event OnComponentHit(CapsuleComponent)
  (params (HitComponent :type Primitive%20Component%20Object%20Reference) (OtherActor :type Actor%20Object%20Reference) (OtherComp :type Primitive%20Component%20Object%20Reference) (NormalImpulse :type Vector :default "0, 0, 0") (Hit :type Hit%20Result%20Structure%20%28by%20ref%29))
  ;[0.15 0.15 0.15 0.5] Dash
  (Utilities|Casting|CastToBP_player OtherActor)
  (if (and (Variables|Default|GetisDashing) (!= (Variables|Default|GetotherIsFlying) true))
    (Variables|Default|SetotherIsFlying true)
    (CallFunction|ExitDash)
    (Default|TakeDamage (Variables|Default|Getplayer) 2)
    (Variables|/Script/Engine.CharacterMovementComponent|SetBrakingFrictionFactor (Variables|Character|GetCharacterMovement) 0.0)
    (bind _returnvalue (Utilities|Time|SetTimerbyEvent (delegate Custom|ApplyLaunchToOther) 0.02 true))
    (Utilities|FlowControl|Delay 0.6)
    (Utilities|Time|PauseTimerbyHandle _returnvalue)
    (Variables|/Script/Engine.CharacterMovementComponent|SetBrakingFrictionFactor (Variables|Character|GetCharacterMovement) 1.0)
    (Variables|Default|SetotherIsFlying false)))

(event Custom|ExitDash
  ;[0.15 0.15 0.15 0.5] Dash
  (Utilities|Time|PauseTimerbyHandle (Variables|Default|GetlaunchTimer))
  (Variables|/Script/Engine.CharacterMovementComponent|SetBrakingFrictionFactor (Variables|Character|GetCharacterMovement) 1.0)
  (Variables|Default|SetisDashing false)
  (Utilities|FlowControl|Delay 1.0)
  (CallFunction|EnableMovement)
  (Utilities|FlowControl|Delay (Math|Random|RandomFloatinRange 0.0 1.0))
  (Variables|Default|SetcanAttack true))

(event Custom|ApplyLaunchToSelf
  ;[0.15 0.15 0.15 0.5] Dash
  (Character|LaunchCharacter (* (Math|Vector|GetForwardVector (Variables|Default|GetCapsuleComponent)) (Variables|Default|GetdashStrength)) true true))

(event Custom|Dash
  ;[0.15 0.15 0.15 0.5] Dash
  (Variables|Default|SetisDashing true)
  (CallFunction|DisableMovement)
  (Variables|/Script/Engine.CharacterMovementComponent|SetBrakingFrictionFactor (Variables|Character|GetCharacterMovement) 0.0)
  (bind _returnvalue (Utilities|Time|SetTimerbyEvent (delegate Custom|ApplyLaunchToSelf) 0.02 true))
  (Variables|Default|SetlaunchTimer _returnvalue)
  (if (Variables|Default|GetisDashing)
    (Utilities|FlowControl|Delay 1.2)
    (CallFunction|ExitDash)))

(event Custom|ApplyLaunchToOther
  ;[0.15 0.15 0.15 0.5] Dash
  (Character|LaunchCharacter (Variables|Default|Getplayer) (* (+ (Math|Vector|GetForwardVector (Variables|Default|GetCapsuleComponent)) (* (Math|Vector|VectorUp) 1.5)) (* (Variables|Default|GetdashStrength) 0.3)) true true))

(event Custom|UseHammer
  ;[0.15 0.15 0.15 0.5] Hammer
  (Development|PrintText "Hammer")
  (Default|Shoot (Variables|Default|Gethammer) (Math|Vector|GetForwardVector (Transformation|GetWorldRotation (Variables|Default|GetGC_Cube))))
  (Utilities|FlowControl|Delay (Math|Random|RandomFloatinRange 2.0 2.5))
  (Variables|Default|SetcanAttack true))

(event Custom|CreateHammer
  ;[0.15 0.15 0.15 0.5] Hammer
  (bind _returnvalue (Game|SpawnActorfromClass "/Game/EnemyBlueprints/BP_HammerBoss.BP_HammerBoss_C" (Math|Transform|MakeTransform (+ (.location (Transformation|GetActorTransform)) (* (Math|Vector|GetForwardVector (Transformation|GetWorldRotation (Variables|Default|GetCapsuleComponent))) 1e+02)) (Math|Conversions|RotationFromXVector (Math|Vector|GetForwardVector (Transformation|GetWorldRotation (Variables|Default|GetCapsuleComponent)))) "1.000000,1.000000,1.000000") "Undefined" "MultiplyWithRoot" 0 0))
  (bind _output_get (Variables|Default|Sethammer _returnvalue))
  (Default|SetParent _output_get self))

(event Custom|RotateHammer
  ;[0.15 0.15 0.15 0.5] Hammer
  (Utilities|IsValid (Variables|Default|Gethammer)
    (:Is%20Valid
      (if (not (Variables|/Game/EnemyBlueprints/BP_SledgeHammer.BP_SledgeHammer_C|GetisFlying (Variables|Default|Gethammer)))
        (Transformation|SetActorTransform (Variables|Default|Gethammer) (Math|Transform|MakeTransform (+ (.location (Transformation|GetActorTransform)) (* (Math|Vector|GetForwardVector (Transformation|GetWorldRotation (Variables|Default|GetCapsuleComponent))) 2e+02)) (Math|Conversions|RotationFromXVector (Math|Vector|GetForwardVector (Transformation|GetWorldRotation (Variables|Default|GetCapsuleComponent)))) "1.000000,1.000000,1.000000"))))))

(event EventAttack
  (Utilities|IsValid (Variables|Default|GetHammer)
    (:Is%20Valid
      (if (Variables|/Game/EnemyBlueprints/BP_SledgeHammer.BP_SledgeHammer_C|GethasCaught (Variables|Default|GetHammer))
        (if (Variables|Default|GetcanAttack)
          (Variables|Default|SetcanAttack false)
          (if (>= (Math|Random|RandomIntegerinRange 1 100) 60)
            (CallFunction|Dash)
            (else
              (CallFunction|UseHammer))))))))

(event EventDie
  (Actor|DestroyActor (Variables|Default|Gethammer))
  (|CallParentFunction))

(event EventBeginPlay
  (CallFunction|SetupBase)
  (CallFunction|CreateHammer)
  (Variables|Default|SetrayCastIgnore (Utilities|Array|MakeArray (Variables|Default|Gethammer))))

(event EventTick
  (params (DeltaSeconds :type Float%20%28single-precision%29))
  (CallFunction|OnTickBase)
  (CallFunction|RotateHammer))

(fn ConstructionScript
  (|CallParentFunction))